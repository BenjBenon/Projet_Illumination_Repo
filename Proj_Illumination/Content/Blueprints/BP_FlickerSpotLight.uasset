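; BP_FlickerSpotLight is a spotlight Blueprint that flickers at random, like an unstable lamp.
; From BeginPlay, a self-calling FlickerLoop event alternates a short dark phase with a usually longer lit phase, randomizing both delays and the lit intensity.
; Each switch fires the OnSwitchIntensity dispatcher with a bool for lit or dark, so bound listeners can follow the flicker.
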(event `self.ReceiveBeginPlay`
  (`self.FlickerLoop`))

(event `FlickerLoop`
  (`LightComponent.SetIntensity` (`self.SpotLight`) 0.0)
  (`self.OnSwitchIntensity` false)
  (`KismetSystemLibrary.Delay` (`KismetMathLibrary.RandomFloatInRange` 0.05 0.3))
  (`LightComponent.SetIntensity` (`self.SpotLight`) (`KismetMathLibrary.RandomFloatInRange` 12000.0 60000.0))
  (`self.OnSwitchIntensity` true)
  (`KismetSystemLibrary.Delay` (`KismetMathLibrary.RandomFloatInRange` 0.1 2.0))
  (`self.FlickerLoop`))

(fn `UserConstructionScript`)