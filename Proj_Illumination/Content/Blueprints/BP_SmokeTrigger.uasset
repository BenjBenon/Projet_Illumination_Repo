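; BP_SmokeTrigger is a trigger actor that starts smoke effects and then loads a level when the player character enters its box.
; After a delay, it loops over an actor array, activating each Niagara component and adding a BPI_FadeIn widget per element.
; A second delay, wired inside the loop body, leads to opening Lvl_ThirdPersonBen.
; The Activate function is an unfinished validity-check loop that does nothing.
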(event `self.Box.OnComponentBeginOverlap`
  (params (OverlappedComponent :type "PrimitiveComponent Object Reference") (OtherActor :type "Actor Object Reference") (OtherComp :type "PrimitiveComponent Object Reference") (OtherBodyIndex :type Integer) (bFromSweep :type Boolean) (SweepResult :type "HitResult Structure (by ref)"))
  (cast `/Game/ThirdPerson/Blueprints/BP_ThirdPersonCharacter` OtherActor)
  (`KismetSystemLibrary.Delay` 7.0)
  (for _array_element (`self.Actor`)
    (`ActorComponent.Activate` (`self.GetComponentByClass` _array_element "/Script/Niagara.NiagaraComponent") false)
    (bind _returnvalue (`|CreateWidget` "/Game/BPI_FadeIn.BPI_FadeIn_C"))
    (`UserWidget.AddToViewport` _returnvalue 0)
    (`KismetSystemLibrary.Delay` 10.0)
    (`GameplayStatics.OpenLevelBySoftObjectPtr` "/Game/ThirdPerson/Lvl_ThirdPersonBen.Lvl_ThirdPersonBen")))

(fn `Activate`
  (for _array_element _
    (`/Engine/EditorBlueprintResources/StandardMacros.IsValid` _array_element)))

(fn `UserConstructionScript`)