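; BP_TriggerSwitch is a puzzle switch that cycles a linked light's color and controls a linked door.
; Each call to Action advances an index through four entries, wrapping with modulo, and applies that color from a list to the light.
; When the index matches the winning index, the door rotates instantly to its open rotation; otherwise it returns to its base rotation.
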(fn `Action`
  (bind _currentindex (`self.currentIndex`))
  (`/Engine/EditorBlueprintResources/StandardMacros.IncrementInt` _currentindex
    (:`  `
      (bind _output_get (set `self.currentIndex` (mod _currentindex 4)))
      (`LightComponent.SetLightColor` (`Light.LightComponent` (`self.linkedLight`)) (`KismetMathLibrary.Conv_ColorToLinearColor` (`|GetArrayItem` (`self.listColor`) _output_get)) true)
      (if (== (`self.currentIndex`) (`self.winningIndex`))
        (`self.K2_SetActorRotation` (`self.linkedDoor`) (`self.rotationOpen`) false)
        (else
          (`self.K2_SetActorRotation` (`self.linkedDoor`) (`self.rotationBase`) false))))))

(fn `UserConstructionScript`
  (`parent.UserConstructionScript`))